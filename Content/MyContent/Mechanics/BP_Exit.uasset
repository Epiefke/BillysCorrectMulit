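; Exit door for the spooky maze that serves as the human player's win point.
; On BeginPlay it binds to the game state's open-door event and caches the human pawn.
; Opening swings two door halves apart on a timeline, and the human overlapping the exit ends the game and travels to the humans-win screen.
; Key-count helpers are partly stubbed: the key check's logic is disconnected, and closing only clears the open flag.
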(event `self.ReceiveBeginPlay`
  (bind _asgs_spooky_maze (cast `/Game/MyContent/Core/GS_SpookyMaze` (`GameplayStatics.GetGameState`)))
  (add `/Game/MyContent/Core/GS_SpookyMaze.OnOpenDoor` _asgs_spooky_maze (`|CreateDelegate` :!event `TryOpen`))
  (bind _asbp_chr_sm_human (cast `/Game/MyContent/Characters/BP_CHR_SM_Human` (`GameplayStatics.GetPlayerPawn` 0)))
  (set `self.HumanRef` _asbp_chr_sm_human))

(event `OpenDoor`
  (`KismetSystemLibrary.PrintString` "Swing")
  (bind (_direction _alpha) (`Timeline|TL_DoorSwing`)
    (:`Update`
      (`SceneComponent.K2_SetRelativeRotation` (`self.Transform_L`) (`KismetMathLibrary.RLerp` (struct) (struct :`Yaw` 90.0) _alpha) false false)
      (`SceneComponent.K2_SetRelativeRotation` (`self.Transform_R`) (`KismetMathLibrary.RLerp` (struct) (struct :`Yaw` -90.0) _alpha) false false))))

(event `self.Exit.OnComponentBeginOverlap`
  (params (OverlappedComponent :type "PrimitiveComponent Object Reference") (OtherActor :type "Actor Object Reference") (OtherComp :type "PrimitiveComponent Object Reference") (OtherBodyIndex :type Integer) (bFromSweep :type Boolean) (SweepResult :type "HitResult Structure (by ref)"))
  (if (== OtherActor (`self.HumanRef`))
    (`self.GameWon`)))

(event `GameWon`
  (bind _asbp_game_instance (cast `/Game/MyContent/Core/BP_GameInstance` (`GameplayStatics.GetGameInstance`)))
  (bind _asbp_player_controller_spooky_maze (cast `/Game/MyContent/Player/BP_PlayerController_SpookyMaze` (`GameplayStatics.GetPlayerController` 0)))
  (`/Game/MyContent/Player/BP_PlayerController_SpookyMaze.EndGame` _asbp_player_controller_spooky_maze)
  (`MGGameInstance.TravelToHumansWin` _asbp_game_instance))

(fn `ChangeKeyNeededTotal`
  (bind _output_get (set `self.KeysToUnlock` (- (`self.KeysCollected`) (`self.KeysToUnlock`))))
  (`KismetSystemLibrary.PrintString` (`KismetStringLibrary.Conv_IntToString` _output_get)))

(fn `Close`
  (set `self.IsOpen` false))

(fn `HasCollectedKey`
  (returns (ReturnValue :type Boolean)))

(fn `Open`
  (set `self.IsOpen` true)
  (`self.OpenDoor`)
  (`KismetSystemLibrary.PrintString` "Open"))

(fn `RemoveKey`
  (params (Amount :type Integer))
  (set `self.KeysCollected` (`KismetMathLibrary.Max` (- (`self.KeysCollected`) Amount)))
  (if (not (`self.HasCollectedKey`))
    (`self.Close`)))

(fn `TryOpen`
  (if (not (`self.IsOpen`))
    (`self.Open`)))

(fn `UserConstructionScript`)