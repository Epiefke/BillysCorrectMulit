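; Player controller for the end-of-game lobby, showing the game-end screen and a text chat.
; On BeginPlay the local controller caches the game instance, creates the game-end and chat widgets, and switches to UI-only input; Enter focuses the chat input.
; SR_SendMessage relays chat through every controller in the GameState PlayerArray to OC_UpdateChat, which updates each chat box.
; A separate OnLoginComplete function opens the lobby widget on success, with no caller in this Blueprint.
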(event `self.ReceiveBeginPlay`
  (if (`self.IsLocalPlayerController`)
    (`WidgetBlueprintLibrary.SetInputMode_UIOnlyEx` self null)
    (bind _asbp_game_instance (cast `/Game/MyContent/Core/BP_GameInstance` (`GameplayStatics.GetGameInstance`)))
    (set `self.Game Instance Ref` _asbp_game_instance)
    (if true
      (bind _returnvalue (`|CreateWidget` "/Game/MyContent/UI/BP_UI_GameEnd.BP_UI_GameEnd_C" self))
      (`UserWidget.AddToPlayerScreen` _returnvalue 0)
      (`WidgetBlueprintLibrary.SetInputMode_UIOnlyEx` self _returnvalue)
      (`self.AddChatBox`))))

(event `Key|Enter`
  (params (Key :type "Key Structure"))
  (:`Released`
    (bind _chatref (`self.ChatRef`)
      (:`then`
        (`Widget.SetKeyboardFocus` (`/Game/MyContent/UI/BP_W_Chatbox.ChatInputBox` _chatref)))
      (:`else`))))

(event `SR_SendMessage`
  (params (PlayerName :type Text) (ChatMessage :type Text))
  (for _array_element (`GameStateBase.PlayerArray` (`GameplayStatics.GetGameState`))
    (bind _asbp_lobby_controller_end (cast `/Game/MyContent/Lobby/BP_LobbyController_End` (`PlayerState.GetPlayerController` _array_element)))
    (`self.OC_UpdateChat` _asbp_lobby_controller_end PlayerName ChatMessage)))

(event `OC_UpdateChat`
  (params (PlayerName :type Text) (ChatMessage :type Text))
  (bind _chatref (`self.ChatRef`)
    (:`then`
      (`/Game/MyContent/UI/BP_W_Chatbox.Update_Chat` _chatref PlayerName ChatMessage))
    (:`else`)))

(fn `AddChatBox`
  (bind _returnvalue (`|CreateWidget` "/Game/MyContent/UI/BP_W_Chatbox.BP_W_Chatbox_C" self))
  (set `self.ChatRef` _returnvalue)
  (`UserWidget.AddToPlayerScreen` _returnvalue 0))

(fn `OnLoginComplete`
  (params (Success :type Boolean) (Error :type String))
  (if Success
    (bind _returnvalue (`|CreateWidget` "/Game/MyContent/UI/BP_UI_Lobby.BP_UI_Lobby_C" self))
    (`UserWidget.AddToPlayerScreen` _returnvalue 0)))

(fn `UserConstructionScript`)