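; Player controller for the lobby that shows either the login screen or the lobby UI to the local player.
; On BeginPlay it sets UI-only input, binds to the GameInstance's login-complete event, then creates the lobby or login widget based on login state.
; OnLoginComplete adds the lobby widget on success, without removing the login widget here or handling failures.
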(event `self.ReceiveBeginPlay`
  (if (`self.IsLocalPlayerController`)
    (`WidgetBlueprintLibrary.SetInputMode_UIOnlyEx` self null)
    (bind _asbp_game_instance (cast `/Game/MyContent/Core/BP_GameInstance` (`GameplayStatics.GetGameInstance`)))
    (bind _output_get (set `self.Game Instance Ref` _asbp_game_instance))
    (`|ExecutionSequence`
      (:`then_0`
        (add `/Game/MyContent/Core/BP_GameInstance.OnLoginComplete` (`self.Game Instance Ref`) (`|CreateDelegate` :!event `OnLoginComplete`)))
      (:`then_1`
        (if (`MGGameInstance.IsLoggedIn` _output_get)
          (bind _returnvalue (`|CreateWidget` "/Game/MyContent/UI/BP_UI_Lobby.BP_UI_Lobby_C" self))
          (`UserWidget.AddToPlayerScreen` _returnvalue 0)
          (else
            (bind _returnvalue_2 (`|CreateWidget` "/Game/MyContent/UI/BP_UI_Login.BP_UI_Login_C" self))
            (`UserWidget.AddToPlayerScreen` _returnvalue_2 0)))))))

(fn `OnLoginComplete`
  (params (Success :type Boolean) (Error :type String))
  (if Success
    (bind _returnvalue (`|CreateWidget` "/Game/MyContent/UI/BP_UI_Lobby.BP_UI_Lobby_C" self))
    (`UserWidget.AddToPlayerScreen` _returnvalue 0)))

(fn `UserConstructionScript`)