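; Game mode for the Spooky Maze match that names joining players and starts the game once everyone from the lobby has arrived.
; Each new player's state gets a numbered display name, and the player state count is checked against the game instance's lobby count.
; On a match, one random player state is flagged special and runs PreGameLogin.
; StartGame then runs on every player state, and again after a short delay.
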(event `self.K2_PostLogin`
  (params (NewPlayer :type "PlayerController Object Reference")))

(event `self.HandleStartingNewPlayer`
  (params (NewPlayer :type "PlayerController Object Reference"))
  (bind _playerarray (`GameStateBase.PlayerArray` (`GameplayStatics.GetGameState`)))
  (`parent.HandleStartingNewPlayer` NewPlayer)
  (`|ExecutionSequence`
    (:`then_0`
      (bind _asbp_sm_player_state (cast `/Game/MyContent/Player/BP_SM_PlayerState` (`Controller.PlayerState` NewPlayer)))
      (`/Game/MyContent/Player/BP_SM_PlayerState.Set Player DisplayName` _asbp_sm_player_state (`KismetStringLibrary.Concat_StrStr` "Player " (`KismetStringLibrary.Conv_IntToString` (`GameplayStatics.GetNumPlayerStates`)))))
    (:`then_1`
      (bind _asbp_game_instance (cast `/Game/MyContent/Core/BP_GameInstance` (`GameplayStatics.GetGameInstance`)))
      (if (== (`/Game/MyContent/Core/BP_GameInstance.LobbyPlayerCount` _asbp_game_instance) (`GameplayStatics.GetNumPlayerStates`))
        (`|ExecutionSequence`
          (:`then_0`
            (if (`KismetArrayLibrary.Array_IsNotEmpty` _playerarray)
              (bind _asbp_sm_player_state_2 (cast `/Game/MyContent/Player/BP_SM_PlayerState` (`KismetArrayLibrary.Array_Random` _playerarray)))
              (set `/Game/MyContent/Player/BP_SM_PlayerState.IsSpecial` true _asbp_sm_player_state_2)
              (`/Game/MyContent/Player/BP_SM_PlayerState.PreGame Login` _asbp_sm_player_state_2)))
          (:`then_1`
            (for _array_element (`GameStateBase.PlayerArray` (`GameplayStatics.GetGameState`))
              (bind _asbp_sm_player_state_3 (cast `/Game/MyContent/Player/BP_SM_PlayerState` _array_element))
              (`/Game/MyContent/Player/BP_SM_PlayerState.Start Game` _asbp_sm_player_state_3))
            (`KismetSystemLibrary.Delay` 5.0)
            (for _array_element_2 (`GameStateBase.PlayerArray` (`GameplayStatics.GetGameState`))
              (bind _asbp_sm_player_state_4 (cast `/Game/MyContent/Player/BP_SM_PlayerState` _array_element_2))
              (`/Game/MyContent/Player/BP_SM_PlayerState.Start Game` _asbp_sm_player_state_4))))))))

(fn `UserConstructionScript`)