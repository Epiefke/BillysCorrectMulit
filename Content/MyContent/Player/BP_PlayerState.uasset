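; Player state Blueprint that stores a player's kill count and display name.
; Both values have RepNotify functions that fire update event dispatchers, and their setters fire the same dispatchers right after assignment.
; AddKill increments the count through SetKills, so it also triggers the kills notification.
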(fn `AddKill`
  (`self.SetKills` (+ (`self.Kills`) 1)))

(fn `OnRep_Kills`
  (`self.OnKillsUpdated`))

(fn `OnRep_PlayerDisplayName`
  (`self.OnPlayerDisplayerNameUpdated`))

(fn `SetKills`
  (params (Kills :type Integer))
  (set `self.Kills` Kills)
  (`self.OnKillsUpdated`))

(fn `SetPlayerDisplayName`
  (params (PlayerDisplayName :type String))
  (set `self.PlayerDisplayName` PlayerDisplayName)
  (`self.OnPlayerDisplayerNameUpdated`))

(fn `UserConstructionScript`)