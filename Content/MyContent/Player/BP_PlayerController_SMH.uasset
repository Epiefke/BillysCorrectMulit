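; Player controller for the SM_Human character that sets up Enhanced Input controls and the player HUD.
; On possess, a client event runs ActivateControls, which caches the controlled character and, for the local controller, adds the mapping context and creates the HUD widget.
; A failed pawn cast sets a half-second timer, apparently to retry.
; Move, jump and camera-turn inputs are forwarded to the cached character.
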(event `self.ReceivePossess`
  (params (PossessedPawn :type "Pawn Object Reference"))
  (`self.Client_OnPossess`))

(event `Client_OnPossess`
  (`self.ActivateControls`))

(event `EnhancedInput|/Game/MyContent/Player/Inputs/IA_Move`
  (params (ActionValue :type "Vector2D Structure") (ElapsedSeconds :type "Float (double-precision)") (TriggeredSeconds :type "Float (double-precision)") (InputAction :type "InputAction Object Reference" :default "/Game/MyContent/Player/Inputs/IA_Move.IA_Move"))
  (:`Triggered`
    (`/Game/MyContent/Characters/BP_CHR_SM_Human.Move Player` (`self.Chara Ref`) ActionValue :!label _label))
  (:`Canceled`
    (goto _label))
  (:`Completed`
    (goto _label)))

(event `EnhancedInput|/Game/MyContent/Player/Inputs/IA_Jump`
  (params (ActionValue :type Boolean) (ElapsedSeconds :type "Float (double-precision)") (TriggeredSeconds :type "Float (double-precision)") (InputAction :type "InputAction Object Reference" :default "/Game/MyContent/Player/Inputs/IA_Jump.IA_Jump"))
  (:`Triggered`
    (`/Game/MyContent/Characters/BP_CHR_SM_Human.Try Jump` (`self.Chara Ref`) ActionValue)))

(event `EnhancedInput|/Game/MyContent/Player/Inputs/IA_TurnCamera`
  (params (ActionValue :type "Vector2D Structure") (ElapsedSeconds :type "Float (double-precision)") (TriggeredSeconds :type "Float (double-precision)") (InputAction :type "InputAction Object Reference" :default "/Game/MyContent/Player/Inputs/IA_TurnCamera.IA_TurnCamera"))
  (:`Triggered`
    (`/Game/MyContent/Characters/BP_CHR_SM_Human.Rotate Camera` (`self.Chara Ref`) ActionValue :!label _label_2))
  (:`Canceled`
    (goto _label_2))
  (:`Completed`
    (goto _label_2)))

(fn `ActivateControls`
  (bind _asbp_chr_sm_human (cast `/Game/MyContent/Characters/BP_CHR_SM_Human` (`self.K2_GetPawn`))
    (:`then`
      (set `self.Chara Ref` _asbp_chr_sm_human)
      (if (`self.IsLocalPlayerController`)
        (`EnhancedInputSubsystemInterface.AddMappingContext` (subsystem `EnhancedInputLocalPlayerSubsystem`) "/Game/MyContent/Player/Inputs/IMC_CHR_SMH.IMC_CHR_SMH" 0 (struct))
        (bind _returnvalue (`|CreateWidget` "/Game/MyContent/UI/BP_UI_SM_Human.BP_UI_SM_Human_C" self))
        (bind _output_get (set `self.Player HUD` _returnvalue))
        (`UserWidget.AddToPlayerScreen` _output_get 0)))
    (:`CastFailed`
      (`KismetSystemLibrary.K2_SetTimerDelegate` (`|CreateDelegate` :!event `ActivateControls`) 0.5))))

(fn `UserConstructionScript`)