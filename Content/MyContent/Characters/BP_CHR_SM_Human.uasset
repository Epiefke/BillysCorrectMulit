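; Playable human character for a networked spooky maze game, handling movement, camera, jumping and a timer widget added on possession.
; On BeginPlay, the locally controlled authority spawns key pickups at randomly chosen, non-repeating BP_KeySpawner actors.
; Sprint and a one-use trap relay through Server-to-Client events, with delays timing sprint duration and cooldown.
; MC_Teleport moves the character to a random BP_TPLocation; key dropping is an empty stub.
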(event `Server_UpdateRepControlRotation`
  (params (Rotator :type "Rotator Structure"))
  (set `self.RepControlRotation` Rotator))

(event `self.ReceivePossessed`
  (params (NewController :type "Controller Object Reference"))
  (`self.OC_AddTimerWidget`))

(event `OC_AddTimerWidget`
  (bind _returnvalue (`|CreateWidget` "/Game/MyContent/UI/BP_W_Timer.BP_W_Timer_C" (`GameplayStatics.GetPlayerController` 0)))
  (bind _output_get (set `self.TimerDisplayRef` _returnvalue))
  (`UserWidget.AddToViewport` _output_get 0))

(event `MC_Teleport`
  (`self.Teleport`))

(event `self.ReceiveBeginPlay`
  (`|ExecutionSequence`
    (:`then_0`
      (if (and (`self.IsLocallyControlled`) (`self.HasAuthority`))
        (bind _outactors (`GameplayStatics.GetAllActorsOfClass` "/Game/MyContent/Mechanics/BP_KeySpawner.BP_KeySpawner_C"))
        (set `self.KeySpawnLocs` _outactors)
        (for _ (range (+ (`self.KeysInLevel`) 1))
          (bind _output_get (set `self.ChoosenKeySpawner` (`KismetArrayLibrary.Array_Random` (`self.KeySpawnLocs`))))
          (`/Engine/EditorBlueprintResources/StandardMacros.IsValid` _output_get
            (:`Is Valid`
              (`|SpawnActorFromClass` "/Game/MyContent/Pickup/BP_KeyPickup.BP_KeyPickup_C" (`self.GetTransform` _output_get) "Undefined" "MultiplyWithRoot" null null)
              (`KismetArrayLibrary.Array_RemoveItem` (`self.KeySpawnLocs`) (`self.ChoosenKeySpawner`)))))))))

(event `Server_SpawnTrap`
  (params (Class :type "Actor Class Reference") (SpawnTransform :type "Transform Structure"))
  ;[1 1 1] Trap
  (`self.Client_SpawnTrap` Class SpawnTransform))

(event `Server_DropKey`
  (params (Class :type "Actor Class Reference") (SpawnTransform :type "Transform Structure"))
  ;[1 1 1] Trap
)

(event `Client_SpawnTrap`
  (params (Class :type "Actor Class Reference") (SpawnTransform :type "Transform Structure"))
  ;[1 1 1] Trap
  (`|SpawnActorFromClass` Class SpawnTransform "Undefined" "MultiplyWithRoot" null null))

(event `Client_DropKey`
  (params (Class :type "Actor Class Reference") (SpawnTransform :type "Transform Structure"))
  ;[1 1 1] Trap
)

(event `Server_Sprint`
  ;[1 1 1] Sprint
  (`self.Client_Sprint`))

(event `Client_Sprint`
  ;[1 1 1] Sprint
  (if (and (`self.CanSprint`) (`self.SprintStart`))
    (set `self.SprintStart` false)
    (set `CharacterMovementComponent.MaxWalkSpeed` 900.0 (`self.CharacterMovement`))
    (`KismetSystemLibrary.Delay` 3.0)
    (`self.Server_DisableSprint`)))

(event `Server_DisableSprint`
  ;[1 1 1] Sprint
  (`self.Client_DisableSprint`))

(event `Client_DisableSprint`
  ;[1 1 1] Sprint
  (set `self.CanSprint` false)
  (set `CharacterMovementComponent.MaxWalkSpeed` 600.0 (`self.CharacterMovement`))
  (`KismetSystemLibrary.Delay` 10.0)
  (`self.Server_EnableSprint`))

(event `Server_EnableSprint`
  ;[1 1 1] Sprint
  (`self.Client_EnableSprint`))

(event `Client_EnableSprint`
  ;[1 1 1] Sprint
  (set `self.CanSprint` true)
  (set `self.SprintStart` true))

(fn `AbilityOne`
  (params (Activate :type Boolean))
  (bind (_returnvalue_location _returnvalue_rotation) (`KismetMathLibrary.BreakTransform` (`SceneComponent.K2_GetComponentToWorld` (`self.Mesh`))))
  (if (not (`self.TrapUsed`))
    (`self.Server_SpawnTrap` "/Game/MyContent/Mechanics/BP_Trap.BP_Trap_C" (`KismetMathLibrary.MakeTransform` _returnvalue_location _returnvalue_rotation))
    (set `self.TrapUsed` true)
    (bind _asbp_player_controller_spooky_maze (cast `/Game/MyContent/Player/BP_PlayerController_SpookyMaze` (`GameplayStatics.GetPlayerController` 0)))
    (`/Game/MyContent/UI/BP_UI_SM_Human.Update Trap UI` (`/Game/MyContent/Player/BP_PlayerController_SpookyMaze.Player HUD` _asbp_player_controller_spooky_maze))))

(fn `DisableSprint`
  (set `self.CanSprint` false))

(fn `Drop Key`)

(fn `EnableSprint`
  (set `self.CanSprint` true)
  (set `self.SprintStart` true)
  (`KismetSystemLibrary.PrintString` "3"))

(fn `Move Player`
  (params (Axis :type "Vector2D Structure"))
  (bind _output_get (set `self.Axis` Axis))
  (`self.PMoveCharacter` _output_get))

(fn `Rotate Camera`
  (params (Axis :type "Vector2D Structure"))
  (`self.AddControllerYawInput` Axis_X)
  (`self.AddControllerPitchInput` (* Axis_Y -1.0)))

(fn `Sprint`
  (`self.Server_Sprint`))

(fn `Teleport`
  (bind _outactors (`GameplayStatics.GetAllActorsOfClass` "/Game/MyContent/Mechanics/BP_TPLocation.BP_TPLocation_C"))
  (bind _output_get (set `self.TeleportLocation` _outactors))
  (bind _outitem (`KismetArrayLibrary.Array_Random` _output_get))
  (`/Engine/EditorBlueprintResources/StandardMacros.IsValid` _outitem
    (:`Is Valid`
      (`self.K2_SetActorLocation` (`self.K2_GetActorLocation` _outitem) false true))))

(fn `Try Jump`
  (params (Jump :type Boolean))
  (if Jump
    (`self.Jump`)
    (else
      (`self.StopJumping`))))

(fn `UserConstructionScript`)