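; Ghost character Blueprint exposing movement, jump and camera-look functions, with no callers in this file.
; MovePlayer scales each axis separately before PMoveCharacter, TryJump starts or stops jumping, and RotateCamera adds yaw and inverted pitch input.
; A server event stores RepControlRotation, but the authority/remote logic in RotateCamera that would update it is disconnected and never runs.
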(event `Server_UpdateRepControlRotation`
  (params (Rotator :type "Rotator Structure"))
  (set `self.RepControlRotation` Rotator))

(fn `Move Player`
  (params (Axis :type "Vector2D Structure"))
  (bind _output_get (set `self.Axis` Axis))
  (`self.PMoveCharacter` (`KismetMathLibrary.MakeVector2D` (/ (`KismetMathLibrary.BreakVector2D` _output_get) 2.5) (/ (`.Y` (`KismetMathLibrary.BreakVector2D` _output_get)) 1.2))))

(fn `Rotate Camera`
  (params (Axis :type "Vector2D Structure"))
  (`self.AddControllerYawInput` Axis_X)
  (`self.AddControllerPitchInput` (* Axis_Y -1.0)))

(fn `Try Jump`
  (params (Jump :type Boolean))
  (if Jump
    (`self.Jump`)
    (else
      (`self.StopJumping`))))

(fn `UserConstructionScript`)