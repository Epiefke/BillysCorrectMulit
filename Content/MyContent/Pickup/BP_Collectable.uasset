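; BP_Collectable is a pickup actor that adds its value to the player's collectable tally and destroys itself when collected.
; On pickup activation it checks CanBeCollected, then Collect applies the value and calls OnCollect to destroy the actor.
; If CountAsCollectable is set, the value goes to the AC_Collectables component found on player 0's pawn.
; The trigger overlap event is empty, and leftover debug prints remain.
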(event `self.BP_OnActivatePickup`
  (params (pickupActor :type "Actor Object Reference"))
  (if (`self.Can be Collected`)
    (`self.Collect` null)))

(event `self.PickupTrigger.OnComponentBeginOverlap`
  (params (OverlappedComponent :type "PrimitiveComponent Object Reference") (OtherActor :type "Actor Object Reference") (OtherComp :type "PrimitiveComponent Object Reference") (OtherBodyIndex :type Integer) (bFromSweep :type Boolean) (SweepResult :type "HitResult Structure (by ref)")))

(fn `Add Collectable`
  (params (`Collectable Componment` :type "/Game/MyContent/Pickup/AC_Collectables Object Reference"))
  (`/Game/MyContent/Pickup/AC_Collectables.Add Collectable` `Collectable Componment` (`self.CollectableValue`))
  (`KismetSystemLibrary.PrintString` "4"))

(fn `Apply Collectable`
  (bind _returnvalue (`self.GetComponentByClass` (`GameplayStatics.GetPlayerPawn` 0) "/Game/MyContent/Pickup/AC_Collectables.AC_Collectables_C"))
  (if (and (`self.CountAsCollectable`) (`KismetSystemLibrary.IsValid` _returnvalue))
    (`self.Add Collectable` _returnvalue)))

(fn `Collect`
  (params (Actor :type "Actor Object Reference"))
  (`self.Apply Collectable`)
  (`self.On Collect` Actor))

(fn `On Collect`
  (params (Actor :type "Actor Object Reference"))
  (`self.K2_DestroyActor`))

(fn `UserConstructionScript`
  (`parent.UserConstructionScript`))