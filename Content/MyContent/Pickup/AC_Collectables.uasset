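; Actor component for the Spooky Maze human character that tracks collected keys, a single held trap and a count of other collectables.
; Add and drop functions change these values, then push them to the player controller's HUD through update functions gated by per-item show flags.
; On BeginPlay it binds to the character's HUD-loaded event to refresh keys and trap, but not collectables.
; Debug prints remain in the key and collectable paths.
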(event `self.ReceiveBeginPlay`
  (bind _asbp_chr_sm_human (cast `/Game/MyContent/Characters/BP_CHR_SM_Human` (`self.GetOwner`)))
  (add `/Game/MyContent/Characters/BP_CHR_SM_Human.PlayerHUDLoaded` _asbp_chr_sm_human (`|CreateDelegate` :!event `OC_PlayerHUDLoaded`)))

(event `OC_PlayerHUDLoaded`
  (`self.Update Keys UI`)
  (`self.Update Trap UI`))

(fn `Add Collectable`
  (params (Amount :type Integer))
  (set `self.Collectables Collected` (+ (`self.Collectables Collected`) Amount))
  (`self.Update Collectable UI`)
  (`KismetSystemLibrary.PrintString` "5"))

(fn `Add Key`
  (params (Amount :type Integer))
  (set `self.KeysCollected` (+ (`self.KeysCollected`) Amount))
  (`self.Update Keys UI`))

(fn `Add Trap`
  (set `self.TrapCollected` true)
  (`self.Update Trap UI`))

(fn `Drop Key`
  (set `self.KeysCollected` (- (`self.KeysCollected`) 1))
  (`self.Update Keys UI`))

(fn `Drop Trap`
  (set `self.TrapCollected` false)
  (`self.Update Trap UI`))

(fn `Update Collectable UI`
  (if (`self.ShowCollectableUI`)
    (bind _asbp_player_controller_spooky_maze (cast `/Game/MyContent/Player/BP_PlayerController_SpookyMaze` (`GameplayStatics.GetPlayerController` 0)))
    (bind _player_hud (`/Game/MyContent/Player/BP_PlayerController_SpookyMaze.Player HUD` _asbp_player_controller_spooky_maze)
      (:`then`
        (`/Game/MyContent/UI/BP_UI_SM_Human.Update Other Collectable UI` _player_hud (`self.Collectables Collected`))
        (`KismetSystemLibrary.PrintString` "6"))
      (:`else`))
    (else
      (`KismetSystemLibrary.PrintString` "Fail"))))

(fn `Update Keys UI`
  (if (`self.ShowKeysUI`)
    (bind _asbp_player_controller_spooky_maze (cast `/Game/MyContent/Player/BP_PlayerController_SpookyMaze` (`GameplayStatics.GetPlayerController` 0))
      (:`then`
        (bind _player_hud (`/Game/MyContent/Player/BP_PlayerController_SpookyMaze.Player HUD` _asbp_player_controller_spooky_maze)
          (:`then`
            (`/Game/MyContent/UI/BP_UI_SM_Human.Update Key UI` _player_hud (`self.KeysCollected`)))
          (:`else`)))
      (:`CastFailed`
        (`KismetSystemLibrary.PrintString` "Fail" :!label _label)))
    (else
      (goto _label))))

(fn `Update Trap UI`
  (if (`self.ShowTrapUI`)
    (bind _asbp_player_controller_spooky_maze (cast `/Game/MyContent/Player/BP_PlayerController_SpookyMaze` (`GameplayStatics.GetPlayerController` 0)))
    (bind _player_hud (`/Game/MyContent/Player/BP_PlayerController_SpookyMaze.Player HUD` _asbp_player_controller_spooky_maze)
      (:`then`
        (`/Game/MyContent/UI/BP_UI_SM_Human.Update Trap UI` _player_hud (`self.TrapCollected`) "Visible"))
      (:`else`
        (`/Game/MyContent/UI/BP_UI_SM_Human.Update Trap UI` _player_hud false "Hidden")))))